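; BP_Barbarous is a player-controlled character with standard movement, jump, mouse look and a montage-based normal attack.
; Input axes move it relative to control rotation, while an Attack flag blocks re-triggering until the AM_Attack montage completes.
; When a montage notify window ends, the next section is set to a random AttackList entry, varying the swing sequence.
; Capsule overlaps only print debug names.
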(event `InputAxis|Move Forward / Backward`
  (params (AxisValue :type "Float (single-precision)"))
  (bind (_returnvalue_roll _returnvalue_pitch _returnvalue_yaw) (`KismetMathLibrary.BreakRotator` (`self.GetControlRotation`)))
  ;[1 1 1] 코멘트
  (`self.AddMovementInput` (`KismetMathLibrary.GetForwardVector` (`KismetMathLibrary.MakeRotator` 0.0 0.0 _returnvalue_yaw)) AxisValue))

(event `InputAxis|Move Right / Left`
  (params (AxisValue :type "Float (single-precision)"))
  (bind (_returnvalue_roll _returnvalue_pitch _returnvalue_yaw) (`KismetMathLibrary.BreakRotator` (`self.GetControlRotation`)))
  ;[1 1 1] 코멘트
  (`self.AddMovementInput` (`KismetMathLibrary.GetRightVector` (`KismetMathLibrary.MakeRotator` _returnvalue_roll 0.0 _returnvalue_yaw)) AxisValue))

(event `InputAction|Jump`
  (params (Key :type "Key Structure"))
  ;[1 1 1] 코멘트
  (:`Pressed`
    (`self.Jump`))
  (:`Released`
    (`self.StopJumping`)))

(event `InputAxis|Turn Right / Left Mouse`
  (params (AxisValue :type "Float (single-precision)"))
  ;[1 1 1] 코멘트
  (`self.AddControllerYawInput` AxisValue))

(event `InputAxis|Look Up / Down Mouse`
  (params (AxisValue :type "Float (single-precision)"))
  ;[1 1 1] 코멘트
  (`self.AddControllerPitchInput` AxisValue))

(event `InputAction|NormalAttack`
  (params (Key :type "Key Structure"))
  (bind _attacklist (`self.AttackList`))
  (bind _returnvalue (`SkeletalMeshComponent.GetAnimInstance` (`self.Mesh`)))
  (bind _returnvalue_2 (`AnimInstance.GetCurrentActiveMontage` _returnvalue))
  (:`Pressed`
    (if (not (`self.Attack`))
      (`|PlayMontage` (`self.Mesh`) "/Game/Blueprint/AM_Attack.AM_Attack"
        (:`then`
          (set `self.Attack` true))
        (:`OnCompleted`
          (set `self.Attack` false))
        (:`OnNotifyEnd`
          (`AnimInstance.Montage_SetNextSection` _returnvalue (`AnimInstance.Montage_GetCurrentSection` _returnvalue _returnvalue_2) (`|GetArrayItem` _attacklist (`KismetMathLibrary.RandomInteger` (`KismetArrayLibrary.Array_Length` _attacklist))) _returnvalue_2))))))

(event `self.Capsule.OnComponentBeginOverlap`
  (params (OverlappedComponent :type "PrimitiveComponent Object Reference") (OtherActor :type "Actor Object Reference") (OtherComp :type "PrimitiveComponent Object Reference") (OtherBodyIndex :type Integer) (bFromSweep :type Boolean) (SweepResult :type "HitResult Structure (by ref)"))
  (`KismetSystemLibrary.PrintString` (`KismetSystemLibrary.GetDisplayName` OtherComp))
  (if (!= OtherComp self)
    (`KismetSystemLibrary.PrintString` (`KismetSystemLibrary.GetDisplayName` null))))

(fn `UserConstructionScript`)