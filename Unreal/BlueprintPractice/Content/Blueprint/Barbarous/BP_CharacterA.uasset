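; BP_CharacterA is a playable character Blueprint with yaw-relative movement, turning, jumping and a montage-driven normal attack.
; NormalAttack plays the ATTACK montage, with IsAttack blocking retriggering until it completes.
; When a montage notify ends, ComboAttack sets the next section to a random AttackList entry, chaining attacks without further input and ignoring its index argument.
; Capsule overlaps and combo results only print debug strings.
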(event `InputAxis|ForwardMove`
  (params (AxisValue :type "Float (single-precision)"))
  (bind (_returnvalue_roll _returnvalue_pitch _returnvalue_yaw) (`KismetMathLibrary.BreakRotator` (`self.GetControlRotation`)))
  ;[1 1 1] 코멘트
  (`self.AddMovementInput` (`KismetMathLibrary.GetForwardVector` (`KismetMathLibrary.MakeRotator` 0.0 0.0 _returnvalue_yaw)) AxisValue))

(event `InputAxis|TurnRight`
  (params (AxisValue :type "Float (single-precision)"))
  (`self.AddControllerYawInput` AxisValue))

(event `InputAxis|SideMove`
  (params (AxisValue :type "Float (single-precision)"))
  (bind (_returnvalue_roll _returnvalue_pitch _returnvalue_yaw) (`KismetMathLibrary.BreakRotator` (`self.GetControlRotation`)))
  ;[1 1 1] 코멘트
  (`self.AddMovementInput` (`KismetMathLibrary.GetRightVector` (`KismetMathLibrary.MakeRotator` _returnvalue_roll 0.0 _returnvalue_yaw)) AxisValue))

(event `InputAction|Jump`
  (params (Key :type "Key Structure"))
  ;[1 1 1] 코멘트
  (:`Pressed`
    (`self.Jump`))
  (:`Released`
    (`self.StopJumping`)))

(event `InputAction|NormalAttack`
  (params (Key :type "Key Structure"))
  (:`Pressed`
    (if (not (`self.isAttack`))
      (`|PlayMontage` (`self.Mesh`) "/Game/Blueprint/Barbarous/ATTACK.ATTACK"
        (:`then`
          (set `self.isAttack` true))
        (:`OnCompleted`
          (set `self.isAttack` false))
        (:`OnNotifyEnd`
          (bind _newparam (`self.ComboAttack` 0))
          (`KismetSystemLibrary.PrintString` (`KismetStringLibrary.Conv_BoolToString` _newparam)))))))

(event `self.Capsule.OnComponentBeginOverlap`
  (params (OverlappedComponent :type "PrimitiveComponent Object Reference") (OtherActor :type "Actor Object Reference") (OtherComp :type "PrimitiveComponent Object Reference") (OtherBodyIndex :type Integer) (bFromSweep :type Boolean) (SweepResult :type "HitResult Structure (by ref)"))
  (if (not (== OtherActor self))
    (`KismetSystemLibrary.PrintString` "Hello")))

(fn `ComboAttack`
  (params (AttackIndex :type Integer))
  (returns (NewParam :type Boolean))
  (bind _attacklist (`self.AttackList`))
  (bind _returnvalue (`SkeletalMeshComponent.GetAnimInstance` (`self.Mesh`)))
  (bind _returnvalue_2 (`AnimInstance.GetCurrentActiveMontage` _returnvalue))
  (`AnimInstance.Montage_SetNextSection` (`SkeletalMeshComponent.GetAnimInstance` (`self.Mesh`)) (`AnimInstance.Montage_GetCurrentSection` _returnvalue _returnvalue_2) (`|GetArrayItem` _attacklist (`KismetMathLibrary.RandomInteger` (`KismetArrayLibrary.Array_Length` _attacklist))) _returnvalue_2)
  (return false))

(fn `UserConstructionScript`)