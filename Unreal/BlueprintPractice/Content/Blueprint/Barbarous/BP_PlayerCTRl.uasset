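; Player controller that drives click-to-move for the controlled pawn through the SetDestination input.
; Pressing stops current movement, and while held, Tick adds movement input toward the point under the cursor.
; Releasing issues a SimpleMoveToLocation to that point.
; Both paths take the location from a complex Visibility-channel trace under the cursor, without checking that it hit.
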(event `InputAction|SetDestination`
  (params (Key :type "Key Structure"))
  (:`Pressed`
    (set `self.InputPressed` true)
    (`self.StopMovement`))
  (:`Released`
    (set `self.InputPressed` false)
    (`self.MovetoHitLocation` (`self.GetLocationUnderCursor`))))

(event `self.ReceiveTick`
  (params (DeltaSeconds :type "Float (single-precision)"))
  (if (`self.InputPressed`)
    (`self.FollowMouseLocation` (`self.GetLocationUnderCursor`))))

(fn `FollowMouseLocation`
  (params (NewParam :type "Vector Structure"))
  (bind _returnvalue (`self.K2_GetPawn`))
  (`Pawn.AddMovementInput` _returnvalue (`KismetMathLibrary.GetDirectionUnitVector` (`self.K2_GetActorLocation` _returnvalue) NewParam) 1.0 false))

(fn `GetLocationUnderCursor`
  (returns (NewParam :type "Vector Structure"))
  (return (`.Location` (`GameplayStatics.BreakHitResult` (`self.GetHitResultUnderCursorByChannel` "TraceTypeQuery1")))))

(fn `MovetoHitLocation`
  (params (Location :type "Vector Structure"))
  (`AIBlueprintHelperLibrary.SimpleMoveToLocation` self Location))

(fn `UserConstructionScript`)