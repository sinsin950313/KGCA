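; Controller for a warrior in InfinityWarrior that makes its controlled pawn wander around the navmesh.
; MoveAFunc picks a random navigable point within NaviRandomRadius of the pawn and sends it there with SimpleMoveToLocation.
; It runs on BeginPlay, then about every five seconds through a Delay on Tick.
; Unconnected leftover nodes hold an unused target approach with a line trace and a sideways-step test.
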(event `self.ReceiveBeginPlay`
  (`self.MoveAFunc`))

(event `self.ReceiveTick`
  (params (DeltaSeconds :type "Float (single-precision)"))
  (`KismetSystemLibrary.Delay` 5.0)
  (`self.MoveAFunc`))

(fn `MoveAFunc`
  (returns (NewParam :type Boolean))
  ;[1 1 1] 램덤위치로 이동
  (bind (_randomlocation _returnvalue) (`NavigationSystemV1.K2_GetRandomLocationInNavigableRadius` (`self.K2_GetActorLocation` (`self.K2_GetPawn`)) (`self.NaviRandomRadius`) null null))
  (bind _output_get (set `self.Random Location` _randomlocation))
  (`AIBlueprintHelperLibrary.SimpleMoveToLocation` self _output_get)
  (return _returnvalue))

(fn `UserConstructionScript`)