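; AI controller for an InfinityWarrior pawn that wanders between TargetPoints in the level.
; BeginPlay caches all TargetPoints, then MoveBFunc shuffles them and simple-moves to the first, repeating about every 10 seconds through a Delay on Tick.
; Its visibility trace draws persistent debug lines, but the obstacle-based goal selection using it is disconnected.
; MoveAFunc, a random navigable-radius move, is defined but never called here.
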(event `self.ReceiveBeginPlay`
  (bind _outactors (`GameplayStatics.GetAllActorsOfClass` "/Script/Engine.TargetPoint"))
  (set `self.TargetList` _outactors)
  (`self.MoveBFunc`))

(event `self.ReceiveTick`
  (params (DeltaSeconds :type "Float (single-precision)"))
  (`KismetSystemLibrary.Delay` 10.0)
  (`self.MoveBFunc`))

(fn `MoveAFunc`
  (returns (NewParam :type Boolean))
  ;[1 1 1] 램덤위치로 이동
  (bind (_randomlocation _returnvalue) (`NavigationSystemV1.K2_GetRandomLocationInNavigableRadius` (`self.K2_GetActorLocation` (`self.K2_GetPawn`)) (`self.NaviRandomRadius`) null null))
  (bind _output_get (set `self.Random Location` _randomlocation))
  (`AIBlueprintHelperLibrary.SimpleMoveToLocation` self _output_get)
  (return _returnvalue))

(fn `MoveBFunc`
  (bind _returnvalue (`self.K2_GetPawn`))
  (bind _targetlist (`self.TargetList`))
  (bind _returnvalue_2 (`self.K2_GetActorLocation` (`|GetArrayItem` _targetlist)))
  (`/Engine/EditorBlueprintResources/StandardMacros.IsValid` _returnvalue
    (:`Is Valid`
      (`KismetArrayLibrary.Array_Shuffle` _targetlist)
      (bind (_outhit _returnvalue_3) (`KismetSystemLibrary.LineTraceSingle` :`Start` (`self.K2_GetActorLocation` _returnvalue) :`End` _returnvalue_2 :`TraceChannel` "TraceTypeQuery1" :`DrawDebugType` "Persistent"))
      (`AIBlueprintHelperLibrary.SimpleMoveToLocation` self _returnvalue_2))))

(fn `UserConstructionScript`)