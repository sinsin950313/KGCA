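; BP_WarriosRifle is a player character blueprint for a rifle-wielding warrior.
; Input axes drive yaw-relative movement and controller look, and BeginPlay spawns a BP_Rifle attached to the mesh's hand_rSocket.
; Fire calls the rifle's Shot, while Jump and Crouch inputs only set state flags, with a debug print on crouch.
; Zoom calls an empty function, and the Jump and StopJumping calls are unconnected.
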(event `InputAxis|ForwardMove`
  (params (AxisValue :type "Float (single-precision)"))
  (bind (_returnvalue_roll _returnvalue_pitch _returnvalue_yaw) (`KismetMathLibrary.BreakRotator` (`self.GetControlRotation`)))
  ;[1 1 1] 코멘트
  (`self.AddMovementInput` (`KismetMathLibrary.GetForwardVector` (`KismetMathLibrary.MakeRotator` 0.0 0.0 _returnvalue_yaw)) AxisValue))

(event `InputAxis|TurnRight`
  (params (AxisValue :type "Float (single-precision)"))
  ;[1 1 1] 코멘트
  (`self.AddControllerYawInput` AxisValue))

(event `InputAxis|ChangePitch`
  (params (AxisValue :type "Float (single-precision)"))
  ;[1 1 1] 코멘트
  (`self.AddControllerPitchInput` AxisValue))

(event `self.ReceiveBeginPlay`
  ;[1 1 1] 코멘트
  (bind _returnvalue (`|SpawnActorFromClass` "/Game/Weapons/BP_Rifle.BP_Rifle_C" (`self.Spawn Transform`) "Undefined" "OverrideRootScale" null null))
  (bind _output_get (set `self.Rifle` _returnvalue))
  (`self.K2_AttachToComponent` _output_get (`self.Mesh`) "hand_rSocket" "KeepRelative" "KeepRelative" "KeepRelative" true))

(event `InputAxis|SideMove`
  (params (AxisValue :type "Float (single-precision)"))
  (bind (_returnvalue_roll _returnvalue_pitch _returnvalue_yaw) (`KismetMathLibrary.BreakRotator` (`self.GetControlRotation`)))
  ;[1 1 1] 코멘트
  (`self.AddMovementInput` (`KismetMathLibrary.GetRightVector` (`KismetMathLibrary.MakeRotator` _returnvalue_roll 0.0 _returnvalue_yaw)) AxisValue))

(event `InputAction|Jump`
  (params (Key :type "Key Structure"))
  ;[1 1 1] 코멘트
  (:`Pressed`
    (set `self.EnableJump` true))
  (:`Released`
    (set `self.EnableJump` false)))

(event `InputAction|Crouch`
  (params (Key :type "Key Structure"))
  ;[1 1 1] 코멘트
  (:`Released`
    (bind _output_get (set `self.EnableCrouch` (not (`self.EnableCrouch`))))
    (`KismetSystemLibrary.PrintString` (`KismetStringLibrary.Concat_StrStr` "Jump" (`KismetStringLibrary.Conv_BoolToString` _output_get)))))

(event `InputAction|Zoom`
  (params (Key :type "Key Structure"))
  ;[1 1 1] 코멘트
  (:`Pressed`
    (`self.Zoom`)))

(event `InputAction|Fire`
  (params (Key :type "Key Structure"))
  (:`Pressed`
    (`/Game/Weapons/BP_Rifle.Shot` (`self.Rifle`))))

(fn `UserConstructionScript`)

(fn `Zoom`)