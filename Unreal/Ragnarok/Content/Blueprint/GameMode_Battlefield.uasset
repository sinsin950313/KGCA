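; Battlefield GameMode that alternates a timed deploy phase with a battle phase for the player controller and an AI commander adversary.
; Tick starts each deploy timer and notifies both sides of phase changes; during battle it polls both for defeat to end the phase.
; Promotion checks four units share a data table row name, then spawns a friendly combatant from that row's PromotionKey.
; Getters expose phase, timer and both controllers.
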(event `self.ReceiveBeginPlay`
  (`|ExecutionSequence`
    (:`then_0`
      (bind _asplayer_controller_battlefiled_player_controller (cast `/Game/Blueprint/Object/Commander/Player/PlayerController_BattlefiledPlayerController` (`GameplayStatics.GetPlayerController` 0)))
      (set `self.Player` _asplayer_controller_battlefiled_player_controller))
    (:`then_1`
      (bind _outactors (`GameplayStatics.GetAllActorsOfClass` "/Game/Blueprint/Object/Commander/AI/AIController_Commander.AIController_Commander_C"))
      (for _array_element _outactors
        (bind _asaicontroller_commander (cast `/Game/Blueprint/Object/Commander/AI/AIController_Commander` (`AIBlueprintHelperLibrary.GetAIController` _array_element)))
        (set `self.Adversary` _asaicontroller_commander)))))

(event `self.ReceiveTick`
  (params (DeltaSeconds :type "Float (single-precision)"))
  (if (`self.BattlePhase`)
    (`|ExecutionSequence`
      (:`then_0`
        (bind _defeat (`/Game/Blueprint/Object/Commander/Player/PlayerController_BattlefiledPlayerController.IsDefeat` (`self.Player`))))
      (:`then_1`
        (bind _defeat_2 (`/Game/Blueprint/Object/Commander/AI/AIController_Commander.IsDefeat` (`self.Adversary`))))
      (:`then_2`
        (if (or _defeat _defeat_2)
          (set `self.BattlePhase` false))))
    (elif (not (`self.IsDeployPhaseStart`))
      (set `self.IsDeployPhaseStart` true)
      (bind _returnvalue (`KismetSystemLibrary.K2_SetTimerDelegate` (delegate `Battle Phase Start`) (`self.DeployTime`)))
      (set `self.TimerHandle` _returnvalue)
      (`|ExecutionSequence`
        (:`then_0`
          (`/Game/Blueprint/Object/Commander/Interface_Commander.DeployPhaseStart` (`self.Player`)))
        (:`then_1`
          (`/Game/Blueprint/Object/Commander/Interface_Commander.DeployPhaseStart` (`self.Adversary`)))))))

(event `Battle Phase Start`
  (set `self.BattlePhase` true)
  (set `self.IsDeployPhaseStart` false)
  (`|ExecutionSequence`
    (:`then_0`
      (`/Game/Blueprint/Object/Commander/Interface_Commander.BattlePhaseStart` (`self.Player`)))
    (:`then_1`
      (`/Game/Blueprint/Object/Commander/Interface_Commander.BattlePhaseStart` (`self.Adversary`)))))

(fn `GetAdversary`
  (returns (Adversary :type "/Game/Blueprint/Object/Commander/Interface_Commander Interface"))
  (return (`self.Adversary`)))

(fn `GetDeployTimeData`
  (returns (Handle :type "TimerHandle Structure") (DeployTime :type "Float (double-precision)"))
  (return (`self.TimerHandle`) (`self.DeployTime`)))

(fn `GetPlayer`
  (returns (Player :type "/Game/Blueprint/Object/Commander/Interface_Commander Interface"))
  (return (`self.Player`)))

(fn `IsBattlePhase`
  (returns (BattlePhase :type Boolean))
  (return (`self.BattlePhase`)))

(fn `Promotion`
  (params (NewParam :type "/Game/Blueprint/Object/Unit/Character_Combatant Object Reference") (NewParam1 :type "/Game/Blueprint/Object/Unit/Character_Combatant Object Reference") (NewParam2 :type "/Game/Blueprint/Object/Unit/Character_Combatant Object Reference") (NewParam3 :type "/Game/Blueprint/Object/Unit/Character_Combatant Object Reference"))
  (returns (Return :type "/Game/Blueprint/Object/Unit/Character_Combatant Object Reference") (Success :type Boolean))
  (locals (NewLocalVar_0 :type "Transform Structure") (NewLocalVar_1 :type Name :default "NewRow"))
  (bind _datatablename (`/Game/Blueprint/Object/Unit/Character_Combatant.DataTableName` NewParam))
  (`|ExecutionSequence`
    (:`then_0`
      (`/Engine/EditorBlueprintResources/StandardMacros.IsValid` NewParam
        (:`Is Not Valid`
          _)))
    (:`then_1`
      (`/Engine/EditorBlueprintResources/StandardMacros.IsValid` NewParam1
        (:`Is Not Valid`
          _)))
    (:`then_2`
      (`/Engine/EditorBlueprintResources/StandardMacros.IsValid` NewParam2
        (:`Is Not Valid`
          _)))
    (:`then_3`
      (`/Engine/EditorBlueprintResources/StandardMacros.IsValid` NewParam3
        (:`Is Not Valid`
          _)))
    (:`then_4`
      (if (and (== _datatablename (`/Game/Blueprint/Object/Unit/Character_Combatant.DataTableName` NewParam1)) (== _datatablename (`/Game/Blueprint/Object/Unit/Character_Combatant.DataTableName` NewParam2)) (== _datatablename (`/Game/Blueprint/Object/Unit/Character_Combatant.DataTableName` NewParam3)))
        (bind _returnvalue (`|GetDataTableRow` "/Game/Blueprint/Object/Unit/DataTable_UnitInformation.DataTable_UnitInformation" _datatablename)
          (:`then`
            (bind _returnvalue_2 (`|SpawnActorFromClass` "/Game/Blueprint/Object/Unit/Character_Combatant.Character_Combatant_C" (`local.NewLocalVar_0`) "Undefined" "OverrideRootScale" null true (`.PromotionKey_18_E3444463464BE37929C871B84D78A1A3` (break `/Game/Blueprint/Object/Unit/Struct_UnitInformation` _returnvalue)) null))
            (return _returnvalue_2 true)))
        (else
          _))))
  (return null false))

(fn `UserConstructionScript`)