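; Battlefield destination actor with a configurable mesh and scale, applied at construction and again on BeginPlay.
; Until raided, its trigger box reacts to overlapping combatants, and a non-friendly one notifies GameMode_Battlefield and sets the Raided flag.
; The same overlap, from either side, spawns any named special unit at SpawnPoint and registers it with that combatant's commander.
; Friendly overlaps leave Raided unset, so they can spawn repeatedly.
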(event `self.ReceiveBeginPlay`
  (bind _destinationmodel (`self.DestinationModel`))
  (`StaticMeshComponent.SetStaticMesh` _destinationmodel (`self.New Mesh`))
  (`SceneComponent.SetWorldScale3D` _destinationmodel (`self.New Scale`)))

(event `self.TriggerBox.OnComponentBeginOverlap`
  (params (OverlappedComponent :type "PrimitiveComponent Object Reference") (OtherActor :type "Actor Object Reference") (OtherComp :type "PrimitiveComponent Object Reference") (OtherBodyIndex :type Integer) (bFromSweep :type Boolean) (SweepResult :type "HitResult Structure (by ref)"))
  (if (not (`self.Raided`))
    (bind _ascharacter_combatant (cast `/Game/Blueprint/Object/Unit/Character_Combatant` OtherActor))
    (`|ExecutionSequence`
      (:`then_0`
        (bind _friendly (`/Game/Blueprint/Object/Unit/Character_Combatant.IsFriendly` _ascharacter_combatant))
        (if (not _friendly)
          (bind _asgame_mode_battlefield (cast `/Game/Blueprint/GameMode_Battlefield` (`GameplayStatics.GetGameMode`)))
          (`/Game/Blueprint/GameMode_Battlefield.Raided` _asgame_mode_battlefield)
          (set `self.Raided` true)))
      (:`then_1`
        (if (!= (`self.SpecialUnitName`) "None")
          (bind _commander (`/Game/Blueprint/Object/Unit/Character_Combatant.GetCommander` _ascharacter_combatant))
          (bind _returnvalue (`|SpawnActorFromClass` "/Game/Blueprint/Object/Unit/Character_SpecialCombatant.Character_SpecialCombatant_C" (`KismetMathLibrary.MakeTransform` (`SceneComponent.K2_GetComponentLocation` (`self.SpawnPoint`))) "Undefined" "OverrideRootScale" null false (`self.SpecialUnitName`) _commander null))
          (`/Game/Blueprint/Object/Commander/Interface_Commander.AddSpecialUnit` _commander _returnvalue))))))

(fn `IsRaided`
  (returns (Raided :type Boolean))
  (return (`self.Raided`)))

(fn `UserConstructionScript`
  (bind _destinationmodel (`self.DestinationModel`))
  (`StaticMeshComponent.SetStaticMesh` _destinationmodel (`self.New Mesh`))
  (`SceneComponent.SetWorldScale3D` _destinationmodel (`self.New Scale`)))