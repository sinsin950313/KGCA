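; Preview box actor that holds a combatant unit at a spawn point and exposes a camera render of it as a material.
; SetCamera creates a render target for the camera and feeds it into a dynamic material instance returned by GetCameraMaterial.
; SetPreviewUnit replaces any previous unit; FocusOff releases it without destroying it.
; Spawn creates a friendly HumanOneStar combatant, previews it and passes it to the battlefield controller's UnitErase.
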(fn `ClearPreviewUnit`
  (`self.K2_DestroyActor` (`self.PreviewUnit`))
  (set `self.PreviewUnit` null))

(fn `FocusOff`
  (set `self.PreviewUnit` null))

(fn `GetCameraMaterial`
  (returns (NewParam :type "MaterialInstance Object Reference"))
  (return (`self.CameraMaterial`)))

(fn `GetPreviewUnit`
  (returns (SpawnedUnit :type "/Game/Blueprint/Object/Unit/Character_Combatant Object Reference"))
  (return (`self.PreviewUnit`)))

(fn `SetCamera`
  (locals (NewLocalVar_0 :type "SkeletalMesh Object Reference" :default "SkeletalMesh'/Game/Models/Mutant/Mutant.Mutant'"))
  (bind _returnvalue (`KismetRenderingLibrary.CreateRenderTarget2D` 256 256 "RTF_RGBA16f" (struct :`G` 0.114498 :`B` 1.0 :`A` 1.0)))
  (bind _output_get (set `SceneCaptureComponent2D.TextureTarget` _returnvalue (`self.Camera`)))
  (bind _returnvalue_2 (`KismetMaterialLibrary.CreateDynamicMaterialInstance` "/Game/Blueprint/UI/Main/TextureRenderTarget2DMaterial_Preview.TextureRenderTarget2DMaterial_Preview" "None"))
  (bind _output_get_2 (set `self.CameraMaterial` _returnvalue_2))
  (`MaterialInstanceDynamic.SetTextureParameterValue` _returnvalue_2 "Texture" _output_get)
  (`MaterialInstanceDynamic.SetTextureParameterValue` _output_get_2 "Texture" _output_get))

(fn `SetPreviewUnit`
  (params (SpawnedUnit :type "/Game/Blueprint/Object/Unit/Character_Combatant Object Reference"))
  (`/Engine/EditorBlueprintResources/StandardMacros.IsValid` (`self.PreviewUnit`)
    (:`Is Valid`
      (`self.ClearPreviewUnit`))
    (:`Is Not Valid`
      _))
  (`self.K2_SetActorLocation` SpawnedUnit (`SceneComponent.K2_GetComponentLocation` (`self.SpawnPoint`)) false false)
  (set `self.PreviewUnit` SpawnedUnit))

(fn `Spawn`
  (locals (NewLocalVar_1 :type "Transform Structure" :default "0.000000,0.000000,-5000.000000|0.000000,0.000000,-0.000000|1.000000,1.000000,1.000000"))
  (bind _returnvalue (`|GetDataTableRow` "/Game/Blueprint/Object/Unit/DataTable_UnitInformation.DataTable_UnitInformation" "HumanOneStar")
    (:`then`
      (bind _returnvalue_2 (`|SpawnActorFromClass` "/Game/Blueprint/Object/Unit/Character_Combatant.Character_Combatant_C" (`local.NewLocalVar_1`) "Undefined" "OverrideRootScale" null true (`.Key_16_F74F3E3A405ACCCB6F4D889C11EFCA94` (break `/Game/Blueprint/Object/Unit/Struct_UnitInformation` _returnvalue)) null null))
      (`self.SetPreviewUnit` _returnvalue_2)
      (bind _asplayer_controller_battlefiled_player_controller (cast `/Game/Blueprint/Object/Commander/Player/PlayerController_BattlefiledPlayerController` (`GameplayStatics.GetPlayerController` 0)))
      (`/Game/Blueprint/Object/Commander/Interface_Commander.UnitErase` _asplayer_controller_battlefiled_player_controller _returnvalue_2))))

(fn `UserConstructionScript`)