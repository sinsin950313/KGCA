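; Player actor that moves around the level and orders a group of focused units to a point under the cursor, RTS-style.
; Forward and Right axes offset its location along its own vectors by MovementSpeed, without sweep or delta-time scaling.
; Releasing MoveTo sends each entry in FocusedUnits to the complex cursor trace hit location.
; FocusedUnits is only read here, with no selection logic in this Blueprint.
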(event `InputAxis|Forward`
  (params (AxisValue :type "Float (single-precision)"))
  (`self.K2_SetActorLocation` (+ (`self.K2_GetActorLocation`) (* AxisValue (`self.GetActorForwardVector`) (`self.MovementSpeed`)))))

(event `InputAxis|Right`
  (params (AxisValue :type "Float (single-precision)"))
  (`self.K2_SetActorLocation` (+ (`self.K2_GetActorLocation`) (* AxisValue (`self.GetActorRightVector`) (`self.MovementSpeed`)))))

(event `InputAction|MoveTo`
  (params (Key :type "Key Structure"))
  (:`Released`
    (for _array_element (`self.FocusedUnits`)
      (`AIController.MoveToLocation` _array_element (`.Location` (`GameplayStatics.BreakHitResult` (`PlayerController.GetHitResultUnderCursorByChannel` (`GameplayStatics.GetPlayerController` 0) "TraceTypeQuery3" true))) -1.0 true true false true null true))))

(event `InputAction|Order`
  (params (Key :type "Key Structure")))

(fn `UserConstructionScript`)