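; Player pawn for a commander that moves over the level while holding a set Height above the surface below it.
; Forward and Right axis inputs offset its location along the actor's forward and right vectors by MovementSpeed, without delta-time scaling.
; Each Tick traces down on the Visibility channel and snaps the pawn to Height above the hit location, without checking whether the trace hit.
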(event `self.ReceiveTick`
  (params (DeltaSeconds :type "Float (single-precision)"))
  (bind _returnvalue (`self.K2_GetActorLocation`))
  (bind _outhit (`KismetSystemLibrary.LineTraceSingle` _returnvalue (`KismetMathLibrary.MakeVector` (.x _returnvalue) (.y _returnvalue) -9999.0) "TraceTypeQuery1"))
  (`self.K2_SetActorLocation` (`KismetMathLibrary.MakeVector` (.x (`.Location` (`GameplayStatics.BreakHitResult` _outhit))) (.y (`.Location` (`GameplayStatics.BreakHitResult` _outhit))) (+ (.z (`.Location` (`GameplayStatics.BreakHitResult` _outhit))) (`self.Height`)))))

(event `InputAxis|Forward`
  (params (AxisValue :type "Float (single-precision)"))
  (`self.K2_SetActorLocation` (+ (`self.K2_GetActorLocation`) (* AxisValue (`self.GetActorForwardVector`) (`self.MovementSpeed`)))))

(event `InputAxis|Right`
  (params (AxisValue :type "Float (single-precision)"))
  (`self.K2_SetActorLocation` (+ (`self.K2_GetActorLocation`) (* AxisValue (`self.GetActorRightVector`) (`self.MovementSpeed`)))))

(fn `UserConstructionScript`)