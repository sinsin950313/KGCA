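; Player controller for the battlefield that shows the mouse cursor and lets the player select and place combatant units.
; On Pick release, a cursor trace stores the hit Character_Combatant as FocusedUnit, or clears it when the cast fails.
; On Deploy release, a valid FocusedUnit moves instantly, without sweep, to the Visibility trace hit location under the cursor.
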(event `self.ReceiveBeginPlay`
  (set `self.bShowMouseCursor` true))

(event `InputAction|Pick`
  (params (Key :type "Key Structure"))
  (:`Released`
    (`self.Pick`)))

(event `InputAction|Deploy`
  (params (Key :type "Key Structure"))
  (:`Released`
    (`self.Deploy`)))

(fn `Deploy`
  (`/Engine/EditorBlueprintResources/StandardMacros.IsValid` (`self.FocusedUnit`)
    (:`Is Valid`
      (`self.K2_SetActorLocation` (`self.FocusedUnit`) (`.Location` (`GameplayStatics.BreakHitResult` (`self.GetHitResultUnderCursorByChannel` "TraceTypeQuery1"))) false false))))

(fn `Pick`
  (`|ExecutionSequence`
    (:`then_0`
      (bind _ascharacter_combatant (cast `/Game/Blueprint/Unit/Character_Combatant` (`.HitActor` (`GameplayStatics.BreakHitResult` (`self.GetHitResultUnderCursorByChannel` "TraceTypeQuery3"))))
        (:`then`
          _)
        (:`CastFailed`
          _))
      (set `self.FocusedUnit` _ascharacter_combatant))))

(fn `UserConstructionScript`)