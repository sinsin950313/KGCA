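; AI controller for combatant units that starts the combatant behavior tree on possession and holds the unit's current target.
; Each tick it removes invalid entries from the target candidate list while looping over it; nothing here fills that list or picks from it.
; A setter assigns the target, and the fight check reports true only while that target is valid and not dead.
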(event `self.ReceivePossess`
  (params (PossessedPawn :type "Pawn Object Reference"))
  (`self.RunBehaviorTree` "/Game/Blueprint/Unit/BehaviorTree_Combatant.BehaviorTree_Combatant"))

(event `self.ReceiveTick`
  (params (DeltaSeconds :type "Float (single-precision)"))
  (for _array_element (`self.TargetCandidnateList`)
    (`/Engine/EditorBlueprintResources/StandardMacros.IsValid` _array_element
      (:`Is Not Valid`
        (`KismetArrayLibrary.Array_RemoveItem` (`self.TargetCandidnateList`) _array_element)))))

(fn `IsFight`
  (returns (IsFight :type Boolean))
  (bind _istargetdead (`self.IsTargetDead`))
  (return (not _istargetdead)))

(fn `IsTargetDead`
  (returns (IsTargetDead :type Boolean))
  (bind _target (`self.Target`))
  (`/Engine/EditorBlueprintResources/StandardMacros.IsValid` _target
    (:`Is Valid`
      (bind _dead (`/Game/Blueprint/Unit/Character_Combatant.IsDead` _target))
      (return _dead))
    (:`Is Not Valid`
      (return true))))

(fn `SetTarget`
  (params (Target :type "/Game/Blueprint/Unit/Character_Combatant Object Reference"))
  (set `self.Target` Target))

(fn `UserConstructionScript`)