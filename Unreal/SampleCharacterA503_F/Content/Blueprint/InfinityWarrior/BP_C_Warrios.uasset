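; AI controller for the Warrios enemy that runs its behavior tree upon possessing BP_WarriosCharacter_3.
; Perception of Player-tagged actors updates the line-of-sight and PlayerActor blackboard keys, with a delayed timer clearing the target after sight is lost.
; Helper functions move the pawn to a random navigable point or a shuffled TargetList entry, the latter with a debug trace whose result goes unused.
; An older copy of the sight logic remains unconnected.
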(event `self.ReceiveBeginPlay`)

(event `self.ReceivePossess`
  (params (PossessedPawn :type "Pawn Object Reference"))
  (cast `/Game/Blueprint/InfinityWarrior/BP_WarriosCharacter_3` PossessedPawn)
  (`self.RunBehaviorTree` "/Game/Blueprint/InfinityWarrior/C_Warrios/BT_C_Warrios.BT_C_Warrios"))

(event `커스텀이벤트_0`
  (bind _returnvalue (`AIBlueprintHelperLibrary.GetBlackboard` null))
  (`BlackboardComponent.SetValueAsBool` _returnvalue (`self.Key Name`) false)
  (`BlackboardComponent.SetValueAsObject` _returnvalue (`self.Key Name_0`) null))

(event `self.AIPerception.OnTargetPerceptionUpdated`
  (params (Actor :type "Actor Object Reference") (Stimulus :type "AIStimulus Structure"))
  (set `self.TargetActor` Actor)
  (if (`self.ActorHasTag` Actor "Player")
    (if (`.bSuccessfullySensed` (break `AIStimulus` Stimulus))
      (`KismetSystemLibrary.K2_ClearAndInvalidateTimerHandle` (`self.LostSightTimer`))
      (`self.UpdateSightKey` true)
      (`self.UpdateTargetKey` (`self.TargetActor`))
      (else
        (bind _returnvalue (`KismetSystemLibrary.K2_SetTimerDelegate` (delegate `LostSight`) 8.0))
        (set `self.LostSightTimer` _returnvalue)
        (`self.UpdateSightKey` false)))))

(event `LostSight`
  (`self.UpdateTargetKey` null))

(fn `MoveAFunc`
  (returns (NewParam :type Boolean))
  ;[1 1 1] 램덤위치로 이동
  (bind (_randomlocation _returnvalue) (`NavigationSystemV1.K2_GetRandomLocationInNavigableRadius` (`self.K2_GetActorLocation` (`self.K2_GetPawn`)) (`self.NaviRandomRadius`) null null))
  (bind _output_get (set `self.Random Location` _randomlocation))
  (`AIBlueprintHelperLibrary.SimpleMoveToLocation` self _output_get)
  (return _returnvalue))

(fn `MoveBFunc`
  (bind _returnvalue (`self.K2_GetPawn`))
  (bind _targetlist (`self.TargetList`))
  (bind _returnvalue_2 (`self.K2_GetActorLocation` (`|GetArrayItem` _targetlist)))
  (`/Engine/EditorBlueprintResources/StandardMacros.IsValid` _returnvalue
    (:`Is Valid`
      (`KismetArrayLibrary.Array_Shuffle` _targetlist)
      (bind (_outhit _returnvalue_3) (`KismetSystemLibrary.LineTraceSingle` :`Start` (`self.K2_GetActorLocation` _returnvalue) :`End` _returnvalue_2 :`TraceChannel` "TraceTypeQuery1" :`DrawDebugType` "Persistent"))
      (`AIBlueprintHelperLibrary.SimpleMoveToLocation` self _returnvalue_2))))

(fn `UpdateSightKey`
  (params (HasLineOfSight :type Boolean))
  (`BlackboardComponent.SetValueAsBool` (`AIBlueprintHelperLibrary.GetBlackboard` null) "HasLineofSight" HasLineOfSight))

(fn `UpdateTargetKey`
  (params (TargetActor :type "Actor Object Reference"))
  (`BlackboardComponent.SetValueAsObject` (`AIBlueprintHelperLibrary.GetBlackboard` null) "PlayerActor" TargetActor))

(fn `UserConstructionScript`)